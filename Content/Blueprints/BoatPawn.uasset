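; Player-controlled boat pawn with throttle and rudder that build up gradually and drift back toward neutral when input is released.
; The Acceleration axis steps Speed, with slower reverse than forward, and feeds it as movement input along the control rotation's forward vector.
; The Steering axis steps Rudder, which yaws the root component and adds scaled controller yaw, turning the travel direction.
; Steps are fixed per input event without delta-time scaling, so handling depends on frame rate.
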(event EventBeginPlay)

(event Collision|EventActorBeginOverlap
  (params (OtherActor :type Actor%20Object%20Reference)))

(event EventTick
  (params (DeltaSeconds :type Float%20%28single-precision%29)))

(event Input|AxisEvents|InputAxisAcceleration
  (params (AxisValue :type Float%20%28single-precision%29))
  (if (> AxisValue 0.0) ; If W
    (if (>= (Variables|Default|GetSpeed) 1.0) ; If speed max
      _
      (else
        (Variables|Default|SetSpeed (+ (Variables|Default|GetSpeed) 0.005))))
    (Pawn|Input|AddMovementInput (Math|Vector|GetForwardVector (Pawn|GetControlRotation :!class /Script/Engine.Pawn)) (Variables|Default|GetSpeed) false :!label _label)
    (elif (< AxisValue 0.0) ; If S
      (if (<= (Variables|Default|GetSpeed) -0.5) ; If speed max reverse
        (goto _label)
        (else
          (Variables|Default|SetSpeed (- (Variables|Default|GetSpeed) 0.005))
          (goto _label)))
      (elif (> (Variables|Default|GetSpeed) 0.0) ; if speed positive
        (Variables|Default|SetSpeed (- (Variables|Default|GetSpeed) 0.001))
        (goto _label)
        (elif (< (Variables|Default|GetSpeed) 0.0) ; if speed negative
          (Variables|Default|SetSpeed (+ (Variables|Default|GetSpeed) 0.001))
          (goto _label))))))

(event Input|AxisEvents|InputAxisSteering
  (params (AxisValue :type Float%20%28single-precision%29))
  (if (> AxisValue 0.0) ; If W
    (if (>= (Variables|Default|GetRudder) 1.0) ; If rudder max left
      _
      (else
        (Variables|Default|SetRudder (+ (Variables|Default|GetRudder) 0.005))))
    (Transformation|AddWorldRotation (Variables|Default|GetDefaultSceneRoot) (Math|Rotator|MakeRotator 0.0 0.0 (Variables|Default|GetRudder)) false false :!label _label)
    (Pawn|Input|AddControllerYawInput (* (Variables|Default|GetRudder) 0.4))
    (elif (< AxisValue 0.0) ; If S
      (if (<= (Variables|Default|GetRudder) -1.0) ; If rudder max right
        (goto _label)
        (else
          (Variables|Default|SetRudder (- (Variables|Default|GetRudder) 0.005))
          (goto _label)))
      (elif (> (Variables|Default|GetRudder) 0.0) ; if rudder left
        (Variables|Default|SetRudder (- (Variables|Default|GetRudder) 0.001))
        (goto _label)
        (elif (< (Variables|Default|GetRudder) 0.0) ; if rudder right
          (Variables|Default|SetRudder (+ (Variables|Default|GetRudder) 0.001))
          (goto _label))))))

(fn ConstructionScript)